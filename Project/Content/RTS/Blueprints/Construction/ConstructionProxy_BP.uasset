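; Construction proxy Blueprint for the RTS that stands in for a building under construction.
; The construction script applies the display mesh, sets material slot 0, then positions or configures the entrance and collision box from that mesh through shared setup functions.
; Tick calls ConstructionCompleted with itself every frame, with no progress check or delay in this graph.
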(event EventTick
  (params (DeltaSeconds :type Float%20%28single-precision%29))
  (Default|CallConstructionCompleted self))

(fn ConstructionScript
  (bind _staticmesh (Variables|Default|GetStaticMesh))
  (Components|StaticMesh|SetStaticMesh _staticmesh (Variables|Default|GetDisplayMesh))
  (Rendering|Material|SetMaterial _staticmesh 0 0)
  (CallFunction|SetBuildingEntrance (Variables|Default|GetEntrance) (Variables|Default|GetStaticMesh))
  (CallFunction|SetBuildingCollisionBox (Variables|Default|GetCollsion) (Variables|Default|GetStaticMesh)))